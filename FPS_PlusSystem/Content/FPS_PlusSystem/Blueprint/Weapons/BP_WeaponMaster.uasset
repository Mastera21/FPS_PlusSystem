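; Base weapon Blueprint for an FPS with a "Plus System" attachment menu covering scope, barrel, grip and magazine.
; Timeline-driven fire spawns bullets at the muzzle, aimed at a far point along the camera's forward vector, with suppressed or normal sound.
; The menu widget takes over input, and Switch events swap attachment meshes by index, with the barrel setting the suppressor flag.
; Closing the menu saves attachments to a named SaveGame slot, which LoadAttachments restores.
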(event Custom|DisplayPlusSystem
  (bind _returnvalue (Game|GetPlayerController 0))
  ;[0 0.5686 0.6824] Plus System
  (Utilities|FlowControl|Delay 0.2)
  (Input|SetIgnoreLookInput _returnvalue true)
  (bind _returnvalue_2 (UserInterface|CreateWidget "/Game/FPS_PlusSystem/UI/PlusSystemWidget.PlusSystemWidget_C" _returnvalue))
  (bind _output_get (Variables|PlusSystem|SetPlusSystemWidget _returnvalue_2))
  (UserInterface|Viewport|AddtoViewport _output_get 0)
  (Input|SetInputModeGameandUI _returnvalue _output_get "LockInFullscreen" false)
  (Variables|/Script/Engine.PlayerController|SetbShowMouseCursor _returnvalue true))

(event Custom|RemovePlusSystem
  (bind _returnvalue (Game|GetPlayerController 0))
  ;[0 0.5686 0.6824] Plus System
  (Input|ResetIgnoreLookInput _returnvalue)
  (Input|SetInputModeGameOnly _returnvalue)
  (Widget|RemovefromParent (Variables|PlusSystem|GetPlusSystemWidget))
  (Variables|/Script/Engine.PlayerController|SetbShowMouseCursor _returnvalue false)
  ;;[0 0.8627 1] Saving current attachments
  (CallFunction|SaveAttachments (Variables|PlusSystem|GetSaveName)))

(event Custom|SwitchMag
  (bind _mag (Variables|Default|GetMag))
  ;[0.2706 1 0] MagSection
  (switch int (Variables|PlusSystem|GetNumMag)
    (:0
      (Components|StaticMesh|SetStaticMesh _mag 0))
    (:1
      (Components|StaticMesh|SetStaticMesh _mag "/Game/FPS_PlusSystem/FPS_Weapon_Bundle/Weapons/Meshes/AR4/AR-15_Mag.AR-15_Mag"))))

(event Custom|SwitchScope
  (bind _scope (Variables|Default|GetScope))
  ;[1 0 0] ScopeSection
  (switch int (Variables|PlusSystem|GetNumScopes)
    (:0
      (Components|StaticMesh|SetStaticMesh _scope 0))
    (:1
      (Components|StaticMesh|SetStaticMesh _scope "/Game/FPS_PlusSystem/FPS_Weapon_Bundle/Weapons/Meshes/Accessories/SM_T4_Sight.SM_T4_Sight"))
    (:2)))

(event Custom|SwitchBarrels
  (bind _barrel (Variables|Default|GetBarrel))
  ;[0 0.07451 1] BarrelSection
  (switch int (Variables|PlusSystem|GetNumBarrels)
    (:0
      (Components|StaticMesh|SetStaticMesh _barrel 0)
      (Variables|HasSuppressor|SetHasSuppressor false))
    (:1
      (Components|StaticMesh|SetStaticMesh _barrel "/Game/FPS_PlusSystem/FPS_Weapon_Bundle/Weapons/Meshes/Accessories/SM_Suppressor5.SM_Suppressor5")
      (Variables|HasSuppressor|SetHasSuppressor true))
    (:2)))

(event Custom|Fire
  (bind _mesh (Variables|Character|GetMesh))
  (bind _camera (Variables|Default|GetCamera))
  (bind _mesh_2 (Variables|Character|GetMesh))
  (bind _returnvalue (Transformation|GetSocketLocation _mesh_2 "Muzzle"))
  (bind _returnvalue_2 (Transformation|GetWorldLocation _mesh))
  ;[1 0.1602 0] Fire
  (Timeline|Timeline_0 Play
    (:Fire
      (Game|SpawnActorfromClass "/Game/FPS_PlusSystem/Blueprint/Bullets/BP_BulletMaster.BP_BulletMaster_C" (Math|Transform|MakeTransform _returnvalue "0, 0, 0" "1,1,1") "Undefined" 0 (* (Math|Vector|Normalize (- (+ (Transformation|GetWorldLocation _camera) (* (Math|Vector|GetForwardVector _camera) 1e+04)) _returnvalue)) 1e+04) 0)
      ;;[0 0 0] Check for suppressor
      (if (Variables|HasSuppressor|GetHasSuppressor)
        (Audio|PlaySoundatLocation (Variables|Sounds|GetSuppressorSound) _returnvalue_2 "0, 0, 0" 1.0 1.0 0.0 0 0 0)
        (else
          (Audio|PlaySoundatLocation (Variables|Sounds|GetNormalSound) _returnvalue_2 "0, 0, 0" 1.0 1.0 0.0 0 0 0))))))

(event Custom|StopFire
  (bind _mesh (Variables|Character|GetMesh))
  (bind _camera (Variables|Default|GetCamera))
  (bind _mesh_2 (Variables|Character|GetMesh))
  (bind _returnvalue (Transformation|GetSocketLocation _mesh_2 "Muzzle"))
  (bind _returnvalue_2 (Transformation|GetWorldLocation _mesh))
  ;[1 0.1602 0] Fire
  (Utilities|FlowControl|Sequence
    (:then_0
      (Timeline|Timeline_0 SetNewTime
        (:Fire
          (Game|SpawnActorfromClass "/Game/FPS_PlusSystem/Blueprint/Bullets/BP_BulletMaster.BP_BulletMaster_C" (Math|Transform|MakeTransform _returnvalue "0, 0, 0" "1,1,1") "Undefined" 0 (* (Math|Vector|Normalize (- (+ (Transformation|GetWorldLocation _camera) (* (Math|Vector|GetForwardVector _camera) 1e+04)) _returnvalue)) 1e+04) 0)
          ;;[0 0 0] Check for suppressor
          (if (Variables|HasSuppressor|GetHasSuppressor)
            (Audio|PlaySoundatLocation (Variables|Sounds|GetSuppressorSound) _returnvalue_2 "0, 0, 0" 1.0 1.0 0.0 0 0 0)
            (else
              (Audio|PlaySoundatLocation (Variables|Sounds|GetNormalSound) _returnvalue_2 "0, 0, 0" 1.0 1.0 0.0 0 0 0))))))
    (:then_1
      (Timeline|Timeline_0 Stop))))

(event Custom|SwitchGrip
  (bind _grip (Variables|Default|GetGrip))
  ;[1 0.6078 0] GripSection
  (switch int (Variables|PlusSystem|GetNumGrip)
    (:0
      (Components|StaticMesh|SetStaticMesh _grip 0))
    (:1
      (Components|StaticMesh|SetStaticMesh _grip "/Game/FPS_PlusSystem/FPS_Weapon_Bundle/Weapons/Meshes/Accessories/SM_Vertgrip.SM_Vertgrip"))
    (:2)))

(event EventBeginPlay)

(fn ConstructionScript
  (|CallParentFunction))

(fn SaveAttachments
  (params (SaveName :type String))
  (bind _returnvalue (SaveGame|DoesSaveGameExist SaveName))
  (if _returnvalue
    ;[0 0.02001 1] Have save (Loading existing save)
    (bind _returnvalue_2 (SaveGame|LoadGamefromSlot SaveName))
    (Variables|PlusSystem|SetSaveAttachmentsRef _returnvalue_2)
    (else
      ;[1 0 0.03113] Doesnt have save (We are creating save)
      (bind _returnvalue_3 (SaveGame|CreateSaveGameObject "/Game/FPS_PlusSystem/Blueprint/SaveSystem/AttachmentsSave.AttachmentsSave_C"))
      (bind _output_get (Variables|PlusSystem|SetSaveAttachmentsRef _returnvalue_3))))
  (bind _asattachments_save (Utilities|Casting|CastToAttachmentsSave _output_get)
    (:then
      ;[0.102 0.1098 0.1765] Setting variables from (Attachments save) to current attachments
      (Variables|/Game/FPS_PlusSystem/Blueprint/SaveSystem/AttachmentsSave.AttachmentsSave_C|SetScope _asattachments_save (Variables|/Script/Engine.StaticMeshComponent|GetStaticMesh (Variables|Default|GetScope)))
      (Variables|/Game/FPS_PlusSystem/Blueprint/SaveSystem/AttachmentsSave.AttachmentsSave_C|SetBarrel _asattachments_save (Variables|/Script/Engine.StaticMeshComponent|GetStaticMesh (Variables|Default|GetBarrel)))
      (Variables|/Game/FPS_PlusSystem/Blueprint/SaveSystem/AttachmentsSave.AttachmentsSave_C|SetGrip _asattachments_save (Variables|/Script/Engine.StaticMeshComponent|GetStaticMesh (Variables|Default|GetGrip)))
      (Variables|/Game/FPS_PlusSystem/Blueprint/SaveSystem/AttachmentsSave.AttachmentsSave_C|SetHasSuppressor _asattachments_save (Variables|HasSuppressor|GetHasSuppressor))
      (Variables|/Game/FPS_PlusSystem/Blueprint/SaveSystem/AttachmentsSave.AttachmentsSave_C|SetMag _asattachments_save (Variables|/Script/Engine.StaticMeshComponent|GetStaticMesh (Variables|Default|GetMag)))
      ;[0 0.715 1] Save attachments
      (SaveGame|SaveGametoSlot (Variables|PlusSystem|GetSaveAttachmentsRef) SaveName))
    (:CastFailed
      ;[0 0 0] Exception
      (Development|PrintString "ERROR, TO CAST ATTACHMENTS SAVE"))))

(fn LoadAttachments
  (params (NameOfSave :type String))
  ;[0.2661 1 0] Check for save
  (bind _returnvalue (SaveGame|DoesSaveGameExist NameOfSave))
  (if _returnvalue
    (bind _returnvalue_2 (SaveGame|LoadGamefromSlot NameOfSave))
    (bind _asattachments_save (Utilities|Casting|CastToAttachmentsSave _returnvalue_2)
      (:then
        ;[0.102 0.1098 0.1765] Setting saved attachments to current attachments
        (Components|StaticMesh|SetStaticMesh (Variables|Default|GetScope) (Variables|/Game/FPS_PlusSystem/Blueprint/SaveSystem/AttachmentsSave.AttachmentsSave_C|GetScope _asattachments_save))
        (Components|StaticMesh|SetStaticMesh (Variables|Default|GetBarrel) (Variables|/Game/FPS_PlusSystem/Blueprint/SaveSystem/AttachmentsSave.AttachmentsSave_C|GetBarrel _asattachments_save))
        (Components|StaticMesh|SetStaticMesh (Variables|Default|GetGrip) (Variables|/Game/FPS_PlusSystem/Blueprint/SaveSystem/AttachmentsSave.AttachmentsSave_C|GetGrip _asattachments_save))
        (Variables|HasSuppressor|SetHasSuppressor (Variables|/Game/FPS_PlusSystem/Blueprint/SaveSystem/AttachmentsSave.AttachmentsSave_C|GetHasSuppressor _asattachments_save))
        (Components|StaticMesh|SetStaticMesh (Variables|Default|GetMag) (Variables|/Game/FPS_PlusSystem/Blueprint/SaveSystem/AttachmentsSave.AttachmentsSave_C|GetMag _asattachments_save)))
      (:CastFailed
        ;[0 0 0] Exception
        (Development|PrintString "ERROR, TO CAST ATTACHMENTS SAVE")))
    (else
      ;;[0 0 0] Exception
      (Development|PrintString "ERROR, DONST HAVE SAVE"))))